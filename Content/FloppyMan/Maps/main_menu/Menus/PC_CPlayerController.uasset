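; PC_CPlayerController is a player controller that toggles the in-game pause menu when the Pause input is pressed.
; With no menu open, it creates W_PauseMenu, switches to game-and-UI input with a visible cursor, pauses the game and hides the ThirdPersonCharacter HUD.
; With the menu open, it removes and clears the stored widget reference, restores game-only input, hides the cursor, unpauses and shows the HUD again.
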(event `InputAction|Pause` :paused true
  (params (Key :type "Key Structure"))
  (bind _returnvalue (`GameplayStatics.GetPlayerController` 0))
  (bind _returnvalue_2 (`GameplayStatics.GetPlayerController` 0))
  (:`Pressed`
    (`/Engine/EditorBlueprintResources/StandardMacros.IsValid` (`self.PauseUIRef`)
      (:`Is Valid`
        (`Widget.RemoveFromParent` (`self.PauseUIRef`))
        (set `self.PauseUIRef` null)
        (`WidgetBlueprintLibrary.SetInputMode_GameOnly` _returnvalue)
        (set `PlayerController.bShowMouseCursor` false _returnvalue)
        (`GameplayStatics.SetGamePaused` false)
        (`/Game/ThirdPersonBP/Blueprints/ThirdPersonCharacter.ToggleHudOn` (cast `/Game/ThirdPersonBP/Blueprints/ThirdPersonCharacter` (`GameplayStatics.GetPlayerCharacter` 0) :!pure true)))
      (:`Is Not Valid`
        (bind _returnvalue_3 (`|CreateWidget` "/Game/FloppyMan/Maps/main_menu/Menus/W_PauseMenu.W_PauseMenu_C"))
        (bind _output_get (set `self.PauseUIRef` _returnvalue_3))
        (`UserWidget.AddToViewport` _output_get 0)
        (`WidgetBlueprintLibrary.SetInputMode_GameAndUIEx` _returnvalue_2 null)
        (set `PlayerController.bShowMouseCursor` true _returnvalue_2)
        (`GameplayStatics.SetGamePaused` true)
        (`/Game/ThirdPersonBP/Blueprints/ThirdPersonCharacter.ToggleHudOff` (cast `/Game/ThirdPersonBP/Blueprints/ThirdPersonCharacter` (`GameplayStatics.GetPlayerCharacter` 0) :!pure true))))))

(fn `UserConstructionScript`)