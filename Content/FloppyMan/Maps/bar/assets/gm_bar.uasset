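; Game mode Blueprint for the bar map that ends the level once all enemies are killed.
; Each enemy_killed event decrements EnemyCount.
; When the count reaches zero or below, it switches the player to UI-only input, adds the Next_level widget to the viewport and shows the mouse cursor.
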(event `enemy_killed`
  (bind _returnvalue (`GameplayStatics.GetPlayerController` 0))
  (bind _result (`/Engine/EditorBlueprintResources/StandardMacros.DecrementInt` (`self.enemy_count`))
    (:`  `
      (set `self.enemy_count` _result)
      (if (<= (`self.enemy_count`) 0)
        (`WidgetBlueprintLibrary.SetInputMode_UIOnlyEx` _returnvalue null)
        (bind _returnvalue_2 (`|CreateWidget` "/Game/FloppyMan/Maps/bar/assets/next_level.next_level_C"))
        (`UserWidget.AddToViewport` _returnvalue_2 0)
        (set `PlayerController.bShowMouseCursor` true _returnvalue)))))

(fn `UserConstructionScript`)